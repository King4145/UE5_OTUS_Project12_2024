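; Health component that tracks the owning actor's health and broadcasts changes and death.
; On BeginPlay it broadcasts the starting health and binds to the owner's OnTakeAnyDamage event.
; Nonzero damage sets Health to Damage minus Health (operands reversed from usual subtraction), clamped to MaxHealth, and flags negative damage as healing.
; At zero health it fires OnDeath and optionally destroys the owner.
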(event `self.ReceiveBeginPlay`
  (bind _health (`self.health`))
  (`self.OnHealthUpdated` _health (/ _health (`self.MaxHealth`)))
  (add `Actor.OnTakeAnyDamage` (`self.GetOwner`) (`|CreateDelegate` :!event `OnTakeDamage`)))

(fn `OnTakeDamage`
  (params (DamagedActor :type "Actor Object Reference") (Damage :type "Float (single-precision)") (DamageType :type "DamageType Object Reference") (InstigatedBy :type "Controller Object Reference") (DamageCauser :type "Actor Object Reference"))
  (bind _health (`self.health`))
  (if (!= Damage 0.0)
    (set `self.health` (`KismetMathLibrary.FClamp` (- Damage (`self.health`)) 0.0 (`self.MaxHealth`)))
    (`self.OnHealthUpdated` _health (/ _health (`self.MaxHealth`)) (< Damage 0.0))
    (if (<= (`self.health`) 0.0)
      (`self.OnDeath`)
      (if (`self.bAutodestroyOnDeath`)
        (`Actor.K2_DestroyActor` (`self.GetOwner`))))))