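; BP_Component is an unfinished health Blueprint that reacts to damage on the owner of a BPACHealthComponent.
; BeginPlay binds an event to that owner's OnTakeAnyDamage, though the bound target is not shown.
; OnTakeDamage sets Health to zero on any nonzero damage, leaving a clamped Damage plus Health calculation unused.
; CustomEvent, NewFunction and the construction script are empty.
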(event `self.ReceiveBeginPlay`
  (add `self.OnTakeAnyDamage` (`ActorComponent.GetOwner` (`self.BPAC_Health_Component`)) (`|CreateDelegate` :!event `onTakeDamage`)))

(event `CustomEvent`
  (params (DamagedActor :type "Actor Object Reference") (Damage :type "Float (single-precision)") (DamageType :type "DamageType Object Reference") (InstigatedBy :type "Controller Object Reference") (DamageCauser :type "Actor Object Reference")))

(fn `NewFunction`)

(fn `onTakeDamage`
  (params (DamagedActor :type "Actor Object Reference") (Damage :type "Float (single-precision)") (DamageType :type "DamageType Object Reference") (InstigatedBy :type "Controller Object Reference") (DamageCauser :type "Actor Object Reference"))
  (locals (NewLocalVar :type "Float (double-precision)" :default 1.0) (NewLocalVar_0 :type "Float (single-precision)"))
  (if (!= Damage 0.0)
    (set `self.Health` 0.0)))

(fn `UserConstructionScript`)