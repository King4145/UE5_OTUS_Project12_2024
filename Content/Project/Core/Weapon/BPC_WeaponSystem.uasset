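; BPC_WeaponSystem is a weapon component that performs a hitscan line trace when its WeaponFire event runs.
; LineTraceLogic traces on the Visibility channel from player 0's controller eye viewpoint along the view direction, with debug drawing.
; Spread comes from randomizing the trace end point inside a small box at maximum range.
; The hit result is returned but unused by WeaponFire, and both hit and miss branches are empty.
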(event `WeaponFire`
  (`self.LineTraceLogic`))

(fn `LineTraceLogic`
  (returns (Hitresult :type "HitResult Structure"))
  (bind (_outlocation _outrotation) (`Actor.GetActorEyesViewPoint` (`GameplayStatics.GetPlayerController` 0)))
  (bind (_outhit _returnvalue) (`KismetSystemLibrary.LineTraceSingle` :`Start` _outlocation :`End` (`KismetMathLibrary.RandomPointInBoundingBox` (+ _outlocation (* (`KismetMathLibrary.Conv_RotatorToVector` _outrotation) 1000.0)) (5.0 5.0 5.0)) :`TraceChannel` "TraceTypeQuery1" :`DrawDebugType` "ForDuration"))
  (if _returnvalue
    _
    (else
      _))
  (bind _output_get (set `self.HitResult` _outhit))
  (return _output_get))