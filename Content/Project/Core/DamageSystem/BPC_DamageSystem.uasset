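; BPC_DamageSystem is a component that tracks health and death state for its owning actor.
; TakeDamage subtracts damage from current health unless already dead, sets IsDead once health reaches zero or below, and prints health and death to screen.
; GetHealthPercent returns current health as a fraction of max health, with no clamping.
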(event `self.ReceiveBeginPlay`)

(fn `Get Health Percent`
  (returns (HealthPercent :type "Float (double-precision)"))
  (return (/ (`self.Current Health`) (`self.MaxHealth`))))

(fn `TakeDamage`
  (params (DamageAmount :type "Float (double-precision)"))
  (if (not (`self.IsDead`))
    (bind _output_get (set `self.Current Health` (- (`self.Current Health`) DamageAmount)))
    (`KismetSystemLibrary.PrintString` (`KismetStringLibrary.Conv_DoubleToString` _output_get))
    (if (<= (`self.Current Health`) 0.0)
      (set `self.IsDead` true)
      (`KismetSystemLibrary.PrintString` "IsDead" true true (struct :`R` 1.0 :`B` 0.147162 :`A` 1.0)))))